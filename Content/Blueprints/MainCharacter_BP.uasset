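; Player character for a sorting algorithm visualizer, with mouse look and movement along its forward, right and up axes.
; Key 1 shuffles the builder's sorting array and key 2 bubble-sorts it, both through the sorting algorithms object.
; Either key then starts the visualization manager's playback, and its running flag blocks both keys while set.
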(event Input|AxisEvents|InputAxisMoveForward
  (params (AxisValue :type Float%20%28single-precision%29))
  ;[0 0.01562 1] Movement and view
  ;;[1 0.375 0] Keyboard
  (Pawn|Input|AddMovementInput (Transformation|GetActorForwardVector) AxisValue false))

(event Input|AxisEvents|InputAxisMoveRight
  (params (AxisValue :type Float%20%28single-precision%29))
  ;[0 0.01562 1] Movement and view
  ;;[1 0.375 0] Keyboard
  (Pawn|Input|AddMovementInput (Transformation|GetActorRightVector) AxisValue false))

(event Input|AxisEvents|InputAxisTurn
  (params (AxisValue :type Float%20%28single-precision%29))
  ;[0 0.01562 1] Movement and view
  ;;[0.9922 1 0] Mouse
  (Pawn|Input|AddControllerYawInput AxisValue))

(event Input|AxisEvents|InputAxisLookUp
  (params (AxisValue :type Float%20%28single-precision%29))
  ;[0 0.01562 1] Movement and view
  ;;[0.9922 1 0] Mouse
  (Pawn|Input|AddControllerPitchInput AxisValue))

(event Input|AxisEvents|InputAxisMoveUp
  (params (AxisValue :type Float%20%28single-precision%29))
  ;[0 0.01562 1] Movement and view
  ;;[1 0.375 0] Keyboard
  (Pawn|Input|AddMovementInput (Transformation|GetActorUpVector) AxisValue false))

(event Input|KeyboardEvents|2
  (params (Key :type Key%20Structure))
  (bind _returnvalue (Class|MainCharacter|GetVisualizationManager))
  (:Pressed
    (if (not (Class|VisualizationManager|GetbIsRunVisualization _returnvalue))
      (Class|VisualizationManager|SetbIsRunVisualization _returnvalue true)
      (Class|SortingAlgorithms|BubbleSort (Class|MainCharacter|GetSortingAlgorithms) (Variables|/Script/VisualAlgorithms.SortingArrayBuilder|GetSortingArray (Class|MainCharacter|GetSortingArrayBuilder)))
      (Class|VisualizationManager|RunVisualization (Class|MainCharacter|GetVisualizationManager)))))

(event Input|KeyboardEvents|1
  (params (Key :type Key%20Structure))
  (bind _returnvalue (Class|MainCharacter|GetVisualizationManager))
  (:Pressed
    (if (not (Class|VisualizationManager|GetbIsRunVisualization _returnvalue))
      (Class|VisualizationManager|SetbIsRunVisualization _returnvalue true)
      (Class|SortingAlgorithms|ShuffleArray (Class|MainCharacter|GetSortingAlgorithms) (Variables|/Script/VisualAlgorithms.SortingArrayBuilder|GetSortingArray (Class|MainCharacter|GetSortingArrayBuilder)))
      (Class|VisualizationManager|RunVisualization (Class|MainCharacter|GetVisualizationManager)))))

(fn ConstructionScript)